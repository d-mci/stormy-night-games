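; Game mode for MbR eSports that alternates which team joining players are pointed to.
; On PostLogin in the level NewMap, a custom event flips the TeamToJoin boolean on BP_Game_State and prints the new value.
; The mode only toggles that flag and does no team assignment itself; a one-second Delay leading into the toggle is left unconnected.
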(event Custom|CustomEvent_0
  (bind _asbp_game_state (Utilities|Casting|CastToBP_Game_State (Game|GetGameState)))
  (bind _output_get (Variables|/Game/_Blueprints/BP_Game_State.BP_Game_State_C|SetTeamToJoin _asbp_game_state (not (Variables|/Game/_Blueprints/BP_Game_State.BP_Game_State_C|GetTeamToJoin _asbp_game_state))))
  (Development|PrintString (Utilities|String|ToString(Boolean) _output_get)))

(event EventPostLogin
  (params (NewPlayer :type Player%20Controller%20Object%20Reference))
  (bind _returnvalue (Game|GetCurrentLevelName true))
  (if (Utilities|Enum|Equal(Enum) _returnvalue "NewMap")
    (CallFunction|CustomEvent0)))

(fn ConstructionScript)