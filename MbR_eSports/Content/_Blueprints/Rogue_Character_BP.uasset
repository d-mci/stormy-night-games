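; Rogue character Blueprint with prototype health and death logic built on the Stats struct in the player state.
; Pressing 1 runs a health check, which destroys the pawn at a low-health threshold through chained server-named and client-named events, then calls an empty TakeDamage function.
; A separate attack event, uncalled here, decrements Health but rewrites Stats with mostly fixed values.
; Print strings serve as debug feedback.
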(event Custom|Destroy%20Actor%20on%20client
  (params (Actor :type Actor%20Object%20Reference))
  ;[1 1 1] Destory actor
  (Utilities|IsValid Actor ; making sure its not done again if the guys already dead
    (:Is%20Valid
      (Actor|DestroyActor Actor)
      (Development|PrintString "Im dead"))))

(event Custom|Destory%20Actor%20on%20server
  (params (Actor :type Actor%20Object%20Reference))
  ;[1 1 1] Destory actor
  (CallFunction|DestroyActoronClient Actor))

(event Custom|CustomEvent
  (params (attack :type Float%20%28single-precision%29))
  ;[1 1 1] Self harm
  (bind _asplayer_state_bp (Utilities|Casting|CastToplayer_state_BP (Variables|GetPlayerState)))
  (bind _result (Math|Float|DecrementFloat (.health (Variables|/Game/_Blueprints/player_state_BP.player_state_BP_C|GetStats _asplayer_state_bp)))
    (:%20%20
      (bind _output_get (Variables|/Game/_Blueprints/player_state_BP.player_state_BP_C|SetStats _asplayer_state_bp (Utilities|Struct|MakeStats 1e+02 1e+02 1e+02 1e+02 2 2 2 _result 0)))
      (Development|PrintString (Utilities|String|ToString(Float) (.health _output_get))))))

(event Custom|Health%20Check
  ;[1 1 1] Health check
  (bind _asplayer_state_bp (Utilities|Casting|CastToplayer_state_BP (Variables|GetPlayerState)))
  (if (<= (Math|Float|Truncate (.health (Variables|/Game/_Blueprints/player_state_BP.player_state_BP_C|GetStats _asplayer_state_bp))) 90)
    (CallFunction|DestoryActoronServer (Variables|/Script/Engine.PlayerState|GetPawnPrivate _asplayer_state_bp))
    (else
      (Development|PrintString "im okay"))))

(event EventBeginPlay)

(event EventTick
  (params (DeltaSeconds :type Float%20%28single-precision%29))
  ;[1 1 1] Self harm
)

(event Collision|EventActorBeginOverlap
  (params (OtherActor :type Actor%20Object%20Reference)))

(event Input|KeyboardEvents|1
  (params (Key :type Key%20Structure :default "None"))
  ;[1 1 1] Self harm
  (:Pressed
    (Utilities|IsValid (Variables|GetPlayerState)
      (:Is%20Valid
        (CallFunction|HealthCheck)
        (CallFunction|TakeDamage 0.0 2e+01)))))

(fn ConstructionScript)

(fn TakeDamage
  (params (attack1 :type Float%20%28single-precision%29) (attack :type Float%20%28single-precision%29)))