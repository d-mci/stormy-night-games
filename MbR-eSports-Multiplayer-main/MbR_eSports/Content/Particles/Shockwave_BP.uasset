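; Shockwave effect actor that plays a one-shot expanding and fading ring burst, then removes itself.
; On BeginPlay it creates dynamic material instances from RingInst for three ring components.
; The RingScale timeline then sets the actor's scale from one track and drives the "Opac" material parameter on all three rings from another, destroying the actor when it finishes.
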(event EventBeginPlay
  (Utilities|FlowControl|Sequence
    (:then_0
      (bind _returnvalue (Rendering|Material|CreateDynamicMaterialInstance (Variables|Default|GetRing1) 0 "/Game/Particles/ringInst.ringInst" "None" :!class /Script/Engine.PrimitiveComponent)))
    (:then_1
      (bind _returnvalue_2 (Rendering|Material|CreateDynamicMaterialInstance (Variables|Default|GetRing) 0 "/Game/Particles/ringInst.ringInst" "None" :!class /Script/Engine.PrimitiveComponent)))
    (:then_2
      (bind _returnvalue_3 (Rendering|Material|CreateDynamicMaterialInstance (Variables|Default|GetRing2) 0 "/Game/Particles/ringInst.ringInst" "None" :!class /Script/Engine.PrimitiveComponent))
      (bind (_direction _yolo _opacity_track) (Timeline|RingScale Play)
        (:Update
          (Transformation|SetActorTransform (Math|Transform|MakeTransform (Transformation|GetActorLocation) (Transformation|GetActorRotation) _yolo))
          (Rendering|Material|SetScalarParameterValue _returnvalue_2 "Opac" _opacity_track :!class /Script/Engine.MaterialInstanceDynamic))
        (:Finished
          (Actor|DestroyActor))))))

(fn ConstructionScript)