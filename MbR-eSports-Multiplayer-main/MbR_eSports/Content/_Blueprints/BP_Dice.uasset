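; BP_Dice is a physics-simulated die that is thrown and reports the face it lands on.
; RotateDice teleports it to a fixed point and applies forces and spin chosen by Key, including randomised and caller-supplied variants.
; Tick calls Calc when the velocity components sum to zero.
; Calc encodes cube orientation against world up as a lookup key into Arr, setting DiceRoll (zero if unmatched) and IsFinished.
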(event Custom|Calc
  (bind _returnvalue (Math|Vector|MakeVector 0.0 0.0 1.0))
  (bind _arr (Variables|Default|Getarr))
  (bind _cube (Variables|Default|GetCube))
  (bind _returnvalue_2 (Math|Vector|GetForwardVector _cube))
  (bind _returnvalue_3 (Math|Vector|GetRightVector _cube))
  (bind _returnvalue_4 (Math|Vector|GetUpVector _cube))
  (bind _returnvalue_5 (- _returnvalue _returnvalue_2))
  (bind _returnvalue_6 (- _returnvalue _returnvalue_3))
  (bind _returnvalue_7 (- _returnvalue _returnvalue_4))
  (bind _returnvalue_8 (Class|KismetMathLibrary|VectorGetAbsMax _returnvalue_7))
  (bind _returnvalue_9 (Class|KismetMathLibrary|VectorGetAbsMax _returnvalue_5))
  (bind _returnvalue_10 (Class|KismetMathLibrary|VectorGetAbsMax _returnvalue_6))
  (bind _returnvalue_11 (Math|Float|Round _returnvalue_8))
  (bind _returnvalue_12 (Math|Float|Round _returnvalue_9))
  (bind _returnvalue_13 (Math|Float|Round _returnvalue_10))
  (bind _returnvalue_14 (* _returnvalue_11 100))
  (bind _returnvalue_15 (* _returnvalue_13 10))
  (bind _returnvalue_16 (+ _returnvalue_12 _returnvalue_15 _returnvalue_14))
  (bind (_value _returnvalue_17) (Utilities|Map|Find _arr _returnvalue_16))
  ;[1 1 1] Calculate what face is upwards
  (if (<= (Math|Vector|VectorLength (Transformation|GetComponentVelocity _cube)) 0.0)
    (Variables|Default|SetdiceRoll (Utilities|Select :Index (Math|Conversions|ToInteger(Boolean) _returnvalue_17) :Option%200 0 :Option%201 _value))
    (Variables|Default|SetisFinished true)))

(event Collision|EventActorBeginOverlap
  (params (OtherActor :type Actor%20Object%20Reference)))

(event EventTick
  (params (DeltaSeconds :type Float%20%28single-precision%29))
  ;[1 1 1] If the dice has finished moving, calculate
  (bind _returnvalue (Physics|GetPhysicsLinearVelocity (Variables|Default|GetCube) "None"))
  (if (== (+ (.x _returnvalue) (.y _returnvalue) (.z _returnvalue)) 0.0)
    (CallFunction|Calc)))

(fn ConstructionScript)

(fn RotateDice
  (params (key :type Integer) (x :type Float%20%28single-precision%29) (y :type Float%20%28single-precision%29))
  (bind _cube (Variables|Default|GetCube))
  (Transformation|SetActorLocation "-2500.000000,-2000.000000,800.000000" false false)
  (Physics|SetSimulatePhysics _cube true)
  (Physics|SetEnableGravity _cube true)
  (Physics|AddForce _cube "1000.000000, 0,1000.000000" "None" false)
  (switch int key
    (:Default
      (Class|PrimitiveComponent|AddAngularImpulseinDegrees _cube "500.000000,100.000000, 0" "None" true :!label _label)
      (Physics|AddImpulse _cube (Math|Vector|MakeVector 0.0 0.0 4e+03) "None" false :!label _label_2)
      (Class|PrimitiveComponent|AddTorqueinDegrees _cube "0,1000.000000,1000.000000" "None" true))
    (:0
      (goto _label))
    (:1
      (Class|PrimitiveComponent|AddAngularImpulseinDegrees _cube "0.000000,600.000000,0.000000" "None" true)
      (goto _label_2))
    (:2
      (Class|PrimitiveComponent|AddAngularImpulseinDegrees _cube (Math|Vector|MakeVector x y 0.0) "None" true))
    (:3
      (Class|PrimitiveComponent|AddAngularImpulseinDegrees _cube (Math|Vector|MakeVector -6e+02 (Math|Random|RandomFloatinRange -2e+02 -6e+02) 1e+03) "None" true)
      (goto _label_2))))