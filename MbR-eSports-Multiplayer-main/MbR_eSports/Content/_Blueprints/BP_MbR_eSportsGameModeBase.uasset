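; Game mode for a tile-based, two-team match that spawns the characters and starts play.
; On BeginPlay it spawns a Mage, Ranger and Rogue for each team at preset spawn transforms, setting each one's team flag and hardcoded starting tile index in opposite corners of the grid.
; A separate Startgame event finds every Player_controller_BP and calls StartGame on it.
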(event Custom|Spawn%20Characters
  ;[1 1 1] spawn other class characters
  (bind _returnvalue (Game|SpawnActorfromClass "/Game/_Blueprints/Player/ThirdPersonBP/Blueprints/MageClass.MageClass_C" (Variables|Default|GetTeam0Spawn1) "Undefined" 0 0))
  (Variables|/Game/_Blueprints/Player/ThirdPersonBP/Blueprints/ThirdPersonCharacter.ThirdPersonCharacter_C|SetTeam _returnvalue true)
  (Variables|/Game/_Blueprints/Player/ThirdPersonBP/Blueprints/ThirdPersonCharacter.ThirdPersonCharacter_C|SetCharacterTileIndex _returnvalue (Utilities|Struct|MakeIntPoint 2 29))
  (bind _returnvalue_2 (Game|SpawnActorfromClass "/Game/_Blueprints/Player/ThirdPersonBP/Blueprints/RangerClass.RangerClass_C" (Variables|Default|GetTeam0Spawn2) "Undefined" 0 0))
  (Variables|/Game/_Blueprints/Player/ThirdPersonBP/Blueprints/ThirdPersonCharacter.ThirdPersonCharacter_C|SetTeam _returnvalue_2 true)
  (Variables|/Game/_Blueprints/Player/ThirdPersonBP/Blueprints/ThirdPersonCharacter.ThirdPersonCharacter_C|SetCharacterTileIndex _returnvalue_2 (Utilities|Struct|MakeIntPoint 2 27))
  (bind _returnvalue_3 (Game|SpawnActorfromClass "/Game/_Blueprints/Player/ThirdPersonBP/Blueprints/RogueClass.RogueClass_C" (Variables|Default|GetTeam0Spawn3) "Undefined" 0 0))
  (Variables|/Game/_Blueprints/Player/ThirdPersonBP/Blueprints/ThirdPersonCharacter.ThirdPersonCharacter_C|SetTeam _returnvalue_3 true)
  (Variables|/Game/_Blueprints/Player/ThirdPersonBP/Blueprints/ThirdPersonCharacter.ThirdPersonCharacter_C|SetCharacterTileIndex _returnvalue_3 (Utilities|Struct|MakeIntPoint 2 25))
  (bind _returnvalue_4 (Game|SpawnActorfromClass "/Game/_Blueprints/Player/ThirdPersonBP/Blueprints/MageClass.MageClass_C" (Variables|Default|GetTeam1Spawn1) "Undefined" 0 0))
  (Variables|/Game/_Blueprints/Player/ThirdPersonBP/Blueprints/ThirdPersonCharacter.ThirdPersonCharacter_C|SetTeam _returnvalue_4 false)
  (Variables|/Game/_Blueprints/Player/ThirdPersonBP/Blueprints/ThirdPersonCharacter.ThirdPersonCharacter_C|SetCharacterTileIndex _returnvalue_4 (Utilities|Struct|MakeIntPoint 29 2))
  (bind _returnvalue_5 (Game|SpawnActorfromClass "/Game/_Blueprints/Player/ThirdPersonBP/Blueprints/RangerClass.RangerClass_C" (Variables|Default|GetTeam1Spawn2) "Undefined" 0 0))
  (Variables|/Game/_Blueprints/Player/ThirdPersonBP/Blueprints/ThirdPersonCharacter.ThirdPersonCharacter_C|SetTeam _returnvalue_5 false)
  (Variables|/Game/_Blueprints/Player/ThirdPersonBP/Blueprints/ThirdPersonCharacter.ThirdPersonCharacter_C|SetCharacterTileIndex _returnvalue_5 (Utilities|Struct|MakeIntPoint 27 2))
  (bind _returnvalue_6 (Game|SpawnActorfromClass "/Game/_Blueprints/Player/ThirdPersonBP/Blueprints/RogueClass.RogueClass_C" (Variables|Default|GetTeam1Spawn3) "Undefined" 0 0))
  (Variables|/Game/_Blueprints/Player/ThirdPersonBP/Blueprints/ThirdPersonCharacter.ThirdPersonCharacter_C|SetTeam _returnvalue_6 false)
  (Variables|/Game/_Blueprints/Player/ThirdPersonBP/Blueprints/ThirdPersonCharacter.ThirdPersonCharacter_C|SetCharacterTileIndex _returnvalue_6 (Utilities|Struct|MakeIntPoint 25 2)))

(event Custom|Start%20game
  ;[1 1 1] start game
  (bind _outactors (Actor|GetAllActorsOfClass "/Game/_Blueprints/player_controller_BP.player_controller_BP_C"))
  (Default|StartGame _outactors))

(event EventBeginPlay
  ;[1 1 1] spawn other class characters
  (CallFunction|SpawnCharacters))

(fn ConstructionScript)