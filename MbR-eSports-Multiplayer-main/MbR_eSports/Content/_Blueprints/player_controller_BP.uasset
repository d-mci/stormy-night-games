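; Player controller for a turn-based, two-team multiplayer game played by clicking tiles to move.
; On NewMap it shows the cursor and copies the game state's TeamToJoin into the player state's Team.
; Clicking a Tile_BP moves the pawn there if its team matches TeamToMove, then EndTurn flips the turn.
; Authority switches and events handle networking, alongside debug keys for ending turns and printing teams; team-swap input is disconnected.
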(event Custom|switchTeam
  ;[1 1 1] Dev Tools
  ;;[1 1 1] Spacebar Swaps Team (on server)
  (bind _asplayer_state_bp (Utilities|Casting|CastToplayer_state_BP (Variables|Default|GetPlayerState)))
  (Variables|/Game/_Blueprints/player_state_BP.player_state_BP_C|SetTeam _asplayer_state_bp (not (Variables|/Game/_Blueprints/player_state_BP.player_state_BP_C|GetTeam _asplayer_state_bp)))
  (CallFunction|CustomEvent0))

(event Custom|End%20turn
  ;[1 1 1] Dev Tools
  ;;[1 1 1] Backspace ends turn (on server)
  (bind _asbp_game_state (Utilities|Casting|CastToBP_Game_State (Game|GetGameState)))
  (Variables|/Game/_Blueprints/BP_Game_State.BP_Game_State_C|SetTeamToMove _asbp_game_state (not (Variables|/Game/_Blueprints/BP_Game_State.BP_Game_State_C|GetTeamToMove _asbp_game_state))))

(event Custom|CustomEvent_0
  ;[1 1 1] update HUD multicast
  (bind _asthird_person_character (Utilities|Casting|CastToThirdPersonCharacter (Game|Player|GetPlayerPawn 0)))
  (Default|CallUpdateHUD _asthird_person_character))

(event Custom|SetTeam
  ;[1 1 1] Sets team (player state) to team to join (game state)
  (bind _asplayer_state_bp (Utilities|Casting|CastToplayer_state_BP (Variables|Default|GetPlayerState)))
  (bind _asbp_game_state (Utilities|Casting|CastToBP_Game_State (Game|GetGameState)))
  (Variables|/Game/_Blueprints/player_state_BP.player_state_BP_C|SetTeam _asplayer_state_bp (Variables|/Game/_Blueprints/BP_Game_State.BP_Game_State_C|GetTeamToJoin _asbp_game_state))
  (CallFunction|CustomEvent0))

(event Custom|Move
  (params (NewParam :type Vector))
  ;[1 1 1] Movement
  (bind _canmove (CallFunction|CanMove))
  (if _canmove
    (AI|Navigation|SimpleMovetoLocation self NewParam)
    (CallFunction|EndTurn)))

(event EventBeginPlay
  ;[1 1 1] display HUD & set team
  (bind _returnvalue (Game|GetCurrentLevelName true))
  (if (Utilities|Enum|Equal(Enum) _returnvalue "NewMap")
    (Variables|Default|SetbShowMouseCursor true)
    (CallFunction|SetTeam)
    (Networking|SwitchHasAuthority
      (:Remote
        ;[1 1 1] Sets team (player state) to team to join (game state)
        (bind _asplayer_state_bp (Utilities|Casting|CastToplayer_state_BP (Variables|Default|GetPlayerState)))
        (bind _asbp_game_state (Utilities|Casting|CastToBP_Game_State (Game|GetGameState)))
        (Variables|/Game/_Blueprints/player_state_BP.player_state_BP_C|SetTeam _asplayer_state_bp (Variables|/Game/_Blueprints/BP_Game_State.BP_Game_State_C|GetTeamToJoin _asbp_game_state))
        (CallFunction|CustomEvent0)))))

(event Input|MouseEvents|LeftMouseButton
  (params (Key :type Key%20Structure :default "None"))
  ;[1 1 1] Movement
  (:Pressed
    (Networking|SwitchHasAuthority
      (:Authority
        _)
      (:Remote
        _))
    (bind _astile_bp (Utilities|Casting|CastToTile_BP (.hitactor (.HitResult (Game|Player|GetHitResultUnderCursorbyChannel self "TraceTypeQuery1" true)))))
    (CallFunction|Move (Transformation|GetActorLocation _astile_bp))))

(event Input|KeyboardEvents|SpaceBar
  (params (Key :type Key%20Structure :default "None"))
  ;[1 1 1] Dev Tools
  ;;[1 1 1] Spacebar Swaps Team (on server)
)

(event Input|KeyboardEvents|Backspace
  (params (Key :type Key%20Structure :default "None"))
  ;[1 1 1] Dev Tools
  ;;[1 1 1] Backspace ends turn (on server)
  (:Pressed
    (Development|PrintString "turn ended")
    (Networking|SwitchHasAuthority
      (:Authority
        _)
      (:Remote
        (CallFunction|EndTurn)))
    (bind _asbp_game_state (Utilities|Casting|CastToBP_Game_State (Game|GetGameState)))
    (Variables|/Game/_Blueprints/BP_Game_State.BP_Game_State_C|SetTeamToMove _asbp_game_state (not (Variables|/Game/_Blueprints/BP_Game_State.BP_Game_State_C|GetTeamToMove _asbp_game_state)))))

(event Input|KeyboardEvents|Tab
  (params (Key :type Key%20Structure :default "None"))
  ;[1 1 1] Dev Tools
  ;;[1 1 1] Tab prints teams, ID's and team to move
  (:Pressed
    (bind _asbp_game_state (Utilities|Casting|CastToBP_Game_State (Game|GetGameState)))
    (if (Variables|/Game/_Blueprints/BP_Game_State.BP_Game_State_C|GetTeamToMove _asbp_game_state)
      (Development|PrintString "Blue Teams Turn")
      (else
        (Development|PrintString "Red Teams Turn")))
    (bind _asplayer_state_bp (Utilities|Casting|CastToplayer_state_BP (Variables|Default|GetPlayerState)))
    (if (Variables|/Game/_Blueprints/player_state_BP.player_state_BP_C|GetTeam _asplayer_state_bp)
      (Development|PrintString "Your team: Blue Team")
      (else
        (Development|PrintString "Your team: Red Team")))))

(fn ConstructionScript)

(fn DisplayHUD
  (if (Pawn|IsLocalPlayerController)
    (bind _returnvalue (UserInterface|CreateWidget "/Game/_Blueprints/HUD.HUD_C"))
    (bind _output_get (Variables|Default|SetHUD _returnvalue))
    (UserInterface|Viewport|AddtoViewport _output_get 0)))

(fn CanMove
  (bind _asbp_game_state (Utilities|Casting|CastToBP_Game_State (Game|GetGameState)))
  (bind _asplayer_state_bp (Utilities|Casting|CastToplayer_state_BP (Variables|Default|GetPlayerState)))
  (return (Math|Boolean|Equal(Boolean) (Variables|/Game/_Blueprints/player_state_BP.player_state_BP_C|GetTeam _asplayer_state_bp) (Variables|/Game/_Blueprints/BP_Game_State.BP_Game_State_C|GetTeamToMove _asbp_game_state))))